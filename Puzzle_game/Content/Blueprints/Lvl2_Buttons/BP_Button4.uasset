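; Level 2 button that pitches the pivot of a Turn_Platform4_Blueprint actor between 0 and 45 degrees.
; Box overlap shows or hides a Press_F widget, whose visibility gates the Turn_Platform event.
; A FlipFlop alternates playing and reversing the timeline, with a DoOnce blocking retriggers until it finishes.
; Timeline updates also shift the button mesh, then set its resting height after a delay.
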(event OnComponentBeginOverlap(Box)
  (params (OverlappedComponent :type Primitive%20Component%20Object%20Reference) (OtherActor :type Actor%20Object%20Reference) (OtherComp :type Primitive%20Component%20Object%20Reference) (OtherBodyIndex :type Integer) (bFromSweep :type Boolean) (SweepResult :type Hit%20Result%20Structure%20%28by%20ref%29))
  (Variables|/Script/UMG.Widget|SetVisibility (Variables|Default|GetPress_Ref) "Visible"))

(event OnComponentEndOverlap(Box)
  (params (OverlappedComponent :type Primitive%20Component%20Object%20Reference) (OtherActor :type Actor%20Object%20Reference) (OtherComp :type Primitive%20Component%20Object%20Reference) (OtherBodyIndex :type Integer))
  (Variables|/Script/UMG.Widget|SetVisibility (Variables|Default|GetPress_Ref) "Hidden"))

(event Custom|Turn_Platform
  (if (Widget|IsVisible (Variables|Default|GetPress_Ref))
    (Utilities|FlowControl|DoOnce false :!label _label
      (:Completed
        (Utilities|FlowControl|FlipFlop
          (:A
            (bind _turn_plat (Timeline|Turn_plat_TL PlayFromStart)
              (:Update
                (Transformation|SetRelativeRotation (Variables|/Game/Blueprints/Turn_Platforms/Turn_Platform_Blueprint.Turn_Platform_Blueprint_C|GetPivot (Variables|Default|GetTurn_Platform_Ref)) (Math|Rotator|MakeRotator 0.0 (Math|Float|Lerp 0.0 45.0 _turn_plat) 0.0) false false)
                (Transformation|SetRelativeLocation (Variables|Default|GetButton) (Math|Vector|MakeVector 0.0 0.0 -12.0) false false)
                (Utilities|FlowControl|Delay 1.0)
                (Transformation|SetRelativeLocation (Variables|Default|GetButton) "0.000000,0.000000,-37.000000" false false))
              (:Finished
                (goto _label Reset))))
          (:B
            (Timeline|Turn_plat_TL ReverseFromEnd)))))))

(event EventBeginPlay
  (bind _returnvalue (UserInterface|CreateWidget "/Game/UI/Press_F.Press_F_C"))
  (bind _output_get (Variables|Default|SetPress_Ref _returnvalue))
  (UserInterface|Viewport|AddtoViewport _output_get 0)
  (bind _returnvalue_2 (Actor|GetActorOfClass "/Game/Blueprints/Turn_Platforms/Turn_Platform4_Blueprint.Turn_Platform4_Blueprint_C"))
  (Variables|Default|SetTurn_Platform_Ref _returnvalue_2))

(fn ConstructionScript)