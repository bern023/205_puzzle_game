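; BP_Final_Door is a password-locked final door that slides or moves open on a timeline.
; Its box trigger enables F-key input while BP_Character overlaps, with a FlipFlop toggling the Password_UI widget, cursor and input mode.
; Leaving the box disables input and removes all widgets without resetting the FlipFlop.
; The FinalDoorOpen event drives the door's relative location; nothing in this Blueprint calls it.
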(event OnComponentBeginOverlap(Door_box)
  (params (OverlappedComponent :type Primitive%20Component%20Object%20Reference) (OtherActor :type Actor%20Object%20Reference) (OtherComp :type Primitive%20Component%20Object%20Reference) (OtherBodyIndex :type Integer) (bFromSweep :type Boolean) (SweepResult :type Hit%20Result%20Structure%20%28by%20ref%29))
  ;[1 1 1] Door Password (Bernadette)
  (Utilities|Casting|CastToBP_Character OtherActor)
  (Input|EnableInput (Game|GetPlayerController 0)))

(event OnComponentEndOverlap(Door_box)
  (params (OverlappedComponent :type Primitive%20Component%20Object%20Reference) (OtherActor :type Actor%20Object%20Reference) (OtherComp :type Primitive%20Component%20Object%20Reference) (OtherBodyIndex :type Integer))
  (bind _returnvalue (Game|GetPlayerController 0))
  ;[1 1 1] Door Password (Bernadette)
  (Utilities|Casting|CastToBP_Character OtherActor)
  (Input|DisableInput (Game|GetPlayerController 0))
  (Viewport|RemoveAllWidgets)
  (Input|SetInputModeGameOnly _returnvalue false)
  (Variables|/Script/Engine.PlayerController|SetbShowMouseCursor _returnvalue false))

(event Custom|Final%20Door%20Open
  ;[1 1 1] Door Password (Bernadette)
  (bind _newtrack_0 (Timeline|Final_DoorTL Play)
    (:Update
      (Transformation|SetRelativeLocation (Variables|Default|GetFinal_Door) _newtrack_0 false false))))

(event Input|KeyboardEvents|F
  (params (Key :type Key%20Structure :default "None"))
  (bind _returnvalue (Game|GetPlayerController 0))
  ;[1 1 1] Door Password (Bernadette)
  (:Pressed
    (Utilities|FlowControl|FlipFlop
      (:A
        (bind _returnvalue_2 (UserInterface|CreateWidget "/Game/UI/Password_UI.Password_UI_C"))
        (UserInterface|Viewport|AddtoViewport _returnvalue_2 0)
        (Input|SetInputModeGameandUI _returnvalue _returnvalue_2 "DoNotLock" true false)
        (Variables|/Script/Engine.PlayerController|SetbShowMouseCursor _returnvalue true))
      (:B
        (Viewport|RemoveAllWidgets)
        (Input|SetInputModeGameOnly _returnvalue false)
        (Variables|/Script/Engine.PlayerController|SetbShowMouseCursor _returnvalue false)))))

(fn ConstructionScript)