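; Player character Blueprint that handles movement, jumping, camera look, object grabbing, pausing and interaction through Enhanced Input.
; Grabbing line-traces along the camera's forward vector and holds the hit component with a Physics Handle, updated every Tick until release.
; The pause input toggles a widget, game pause, cursor and input mode.
; Interact calls TurnPlatform on the first actor found of each of five button classes, with no proximity check.
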(event Input|EnhancedActionEvents|EnhancedInputActionINP_Jump
  (params (ActionValue :type Boolean) (ElapsedSeconds :type Float%20%28double-precision%29) (TriggeredSeconds :type Float%20%28double-precision%29) (InputAction :type Input%20Action%20Object%20Reference :default "/Game/Inputs/INP_Jump.INP_Jump"))
  ;[1 1 1] Jump (Bernadette)
  (:Started
    (Character|Jump))
  (:Completed
    (Character|StopJumping)))

(event Input|EnhancedActionEvents|EnhancedInputActionINP_Movement
  (params (ActionValue :type Vector%202D%20Structure) (ElapsedSeconds :type Float%20%28double-precision%29) (TriggeredSeconds :type Float%20%28double-precision%29) (InputAction :type Input%20Action%20Object%20Reference :default "/Game/Inputs/INP_Movement.INP_Movement"))
  (bind _returnvalue (Pawn|GetControlRotation :!class /Script/Engine.Pawn))
  ;[1 1 1] Move around (Bernadette)
  (:Triggered
    (Pawn|Input|AddMovementInput (Math|Vector|GetRightVector (Pawn|GetControlRotation :!class /Script/Engine.Pawn)) (.x ActionValue) false)
    (Pawn|Input|AddMovementInput (Math|Vector|GetForwardVector (Math|Rotator|MakeRotator (.roll _returnvalue) 0.0 (.yaw _returnvalue))) (.y ActionValue) false)))

(event Input|EnhancedActionEvents|EnhancedInputActionINP_LookAround
  (params (ActionValue :type Vector%202D%20Structure) (ElapsedSeconds :type Float%20%28double-precision%29) (TriggeredSeconds :type Float%20%28double-precision%29) (InputAction :type Input%20Action%20Object%20Reference :default "/Game/Inputs/INP_LookAround.INP_LookAround"))
  ;[1 1 1] Look Around (Bernadette)
  (:Triggered
    (Pawn|Input|AddControllerYawInput (* (.x ActionValue) (Math|Float|SelectFloat -1.0 1.0 (Variables|Default|GetInvertCameraX))))
    (Pawn|Input|AddControllerPitchInput (* (.y ActionValue) (Math|Float|SelectFloat -1.0 1.0 (Variables|Default|GetInvertCameraY))))))

(event Input|EnhancedActionEvents|EnhancedInputActionIA_PauseGame
  (params (ActionValue :type Boolean) (ElapsedSeconds :type Float%20%28double-precision%29) (TriggeredSeconds :type Float%20%28double-precision%29) (InputAction :type Input%20Action%20Object%20Reference :default "/Game/Inputs/IA_PauseGame.IA_PauseGame"))
  (bind _returnvalue (Game|GetPlayerController 0))
  ;[1 1 1] Pause and unpause (Bernadette)
  (:Started
    (if (not (Variables|Default|GetIsPauseOpen))
      (Variables|Default|SetIsPauseOpen true)
      (bind _returnvalue_2 (UserInterface|CreateWidget "/Game/UI/Pause.Pause_C" _returnvalue))
      (bind _output_get (Variables|Default|SetPause_Widget _returnvalue_2))
      (UserInterface|Viewport|AddtoViewport _output_get 0)
      (Input|SetInputModeGameandUI _returnvalue (Variables|Default|GetPause_Widget) "DoNotLock" true false)
      (Variables|/Script/Engine.PlayerController|SetbShowMouseCursor (Game|GetPlayerController 0) true)
      (Game|SetGamePaused true)
      (else
        (Variables|Default|SetIsPauseOpen false)
        (Widget|RemovefromParent (Variables|Default|GetPause_Widget))
        (Game|SetGamePaused false)
        (Input|SetInputModeGameOnly _returnvalue false)
        (Variables|/Script/Engine.PlayerController|SetbShowMouseCursor (Game|GetPlayerController 0) false)))))

(event Input|EnhancedActionEvents|EnhancedInputActionINP_Grab
  (params (ActionValue :type Boolean) (ElapsedSeconds :type Float%20%28double-precision%29) (TriggeredSeconds :type Float%20%28double-precision%29) (InputAction :type Input%20Action%20Object%20Reference :default "/Game/Inputs/INP_Grab.INP_Grab"))
  (bind _scene (Variables|Default|GetScene))
  (bind _returnvalue (Transformation|GetWorldLocation _scene))
  ;[1 1 1] Grab Object (Bernadette)
  (:Triggered
    (bind (_outhit _returnvalue_2) (Collision|LineTraceByChannel _returnvalue (+ _returnvalue (* (Math|Vector|GetForwardVector (Variables|Default|GetCharCam)) 3e+02)) "TraceTypeQuery1" false 0 "None"))
    (if _returnvalue_2
      (Physics|Components|PhysicsHandle|GrabComponentatLocationwithRotation (Variables|Default|GetPhysicsHandle) (.HitComponent (Collision|BreakHitResult _outhit)) "None" (Transformation|GetWorldLocation (.HitComponent (Collision|BreakHitResult _outhit))) (Transformation|GetWorldRotation (.HitComponent (Collision|BreakHitResult _outhit))))
      (Variables|Default|SetGrabbingObject true)))
  (:Completed
    (if (Variables|Default|GetGrabbingObject)
      (Physics|Components|PhysicsHandle|ReleaseComponent (Variables|Default|GetPhysicsHandle))
      (Variables|Default|SetGrabbingObject false))))

(event Input|EnhancedActionEvents|EnhancedInputActionINP_Interact
  (params (ActionValue :type Boolean) (ElapsedSeconds :type Float%20%28double-precision%29) (TriggeredSeconds :type Float%20%28double-precision%29) (InputAction :type Input%20Action%20Object%20Reference :default "/Game/Inputs/INP_Interact.INP_Interact"))
  (:Triggered
    (bind _returnvalue (Actor|GetActorOfClass "/Game/Blueprints/Lvl2_Buttons/BP_Button5.BP_Button5_C"))
    (Default|TurnPlatform _returnvalue)))

(event Input|EnhancedActionEvents|EnhancedInputActionINP_Interact
  (params (ActionValue :type Boolean) (ElapsedSeconds :type Float%20%28double-precision%29) (TriggeredSeconds :type Float%20%28double-precision%29) (InputAction :type Input%20Action%20Object%20Reference :default "/Game/Inputs/INP_Interact.INP_Interact"))
  (:Triggered
    (bind _returnvalue (Actor|GetActorOfClass "/Game/Blueprints/Lvl2_Buttons/BP_Button1.BP_Button1_C"))
    (Default|TurnPlatform _returnvalue)))

(event Input|EnhancedActionEvents|EnhancedInputActionINP_Interact
  (params (ActionValue :type Boolean) (ElapsedSeconds :type Float%20%28double-precision%29) (TriggeredSeconds :type Float%20%28double-precision%29) (InputAction :type Input%20Action%20Object%20Reference :default "/Game/Inputs/INP_Interact.INP_Interact"))
  (:Triggered
    (bind _returnvalue (Actor|GetActorOfClass "/Game/Blueprints/Lvl2_Buttons/BP_Button2.BP_Button2_C"))
    (Default|TurnPlatform _returnvalue)))

(event Input|EnhancedActionEvents|EnhancedInputActionINP_Interact
  (params (ActionValue :type Boolean) (ElapsedSeconds :type Float%20%28double-precision%29) (TriggeredSeconds :type Float%20%28double-precision%29) (InputAction :type Input%20Action%20Object%20Reference :default "/Game/Inputs/INP_Interact.INP_Interact"))
  (:Triggered
    (bind _returnvalue (Actor|GetActorOfClass "/Game/Blueprints/Lvl2_Buttons/BP_Button3.BP_Button3_C"))
    (Default|TurnPlatform _returnvalue)))

(event Input|EnhancedActionEvents|EnhancedInputActionINP_Interact
  (params (ActionValue :type Boolean) (ElapsedSeconds :type Float%20%28double-precision%29) (TriggeredSeconds :type Float%20%28double-precision%29) (InputAction :type Input%20Action%20Object%20Reference :default "/Game/Inputs/INP_Interact.INP_Interact"))
  (:Triggered
    (bind _returnvalue (Actor|GetActorOfClass "/Game/Blueprints/Lvl2_Buttons/BP_Button4.BP_Button4_C"))
    (Default|TurnPlatform _returnvalue)))

(event EventBeginPlay
  (bind _returnvalue (Game|GetPlayerController 0))
  (bind _returnvalue_2 (PlayerController|LocalPlayerSubsystems|GetEnhancedInputLocalPlayerSubsystem _returnvalue))
  ;[1 1 1] Animations (Bernadette)
  (Utilities|IsValid _returnvalue_2
    (:Is%20Valid
      (Input|AddMappingContext _returnvalue_2 "/Game/Inputs/IMC_ThirdPerson.IMC_ThirdPerson" 0 "(bIgnoreAllPressedKeysUntilRelease=True,bForceImmediately=False)"))))

(event EventTick
  (params (DeltaSeconds :type Float%20%28single-precision%29))
  (bind _charcam (Variables|Default|GetCharCam))
  ;[1 1 1] Grab Object (Bernadette)
  (if (Variables|Default|GetGrabbingObject)
    (Class|PhysicsHandleComponent|SetTargetLocationandRotation (Variables|Default|GetPhysicsHandle) (+ (Transformation|GetWorldLocation (Variables|Default|GetScene)) (* (Math|Vector|GetForwardVector _charcam) 3e+02)) (Transformation|GetWorldRotation _charcam))))

(fn ConstructionScript)